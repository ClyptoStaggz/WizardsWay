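; BP_Pickup_Coins is a coin pickup that adds one to the player's coin count in the mage runner game.
; On BeginPlay it sets its pickup mesh to a random entry from its Coins array for visual variety.
; When a BP_MageRunner overlaps it, it increments that character's Coins, then passes the overlap to the parent class's handler.
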(event `self.ReceiveBeginPlay`
  (`StaticMeshComponent.SetStaticMesh` (`self.Pickup_Mesh`) (`KismetArrayLibrary.Array_Random` (`self.Coins`))))

(event `self.ReceiveActorBeginOverlap`
  (params (OtherActor :type "Actor Object Reference"))
  (bind _asbp_mage_runner (cast `/Game/Blueprints/BP_MageRunner` OtherActor))
  (`/Engine/EditorBlueprintResources/StandardMacros.IncrementInt` (`/Game/Blueprints/BP_MageRunner.Coins` _asbp_mage_runner)
    (:`  `
      (`parent.ReceiveActorBeginOverlap` OtherActor))))

(fn `UserConstructionScript`
  (`parent.UserConstructionScript`))