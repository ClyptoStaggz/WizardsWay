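; GM_MageRunner is a game mode that lays out a straight track of BP_Block actors at BeginPlay.
; It calls AddBlock AmountOfBlocks times, leaving SpawnStuff off for the first few blocks and on for the rest.
; AddBlock places each block at a fixed spacing along X using the LastBlock counter, then increments that counter.
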(event `self.ReceiveBeginPlay`
  (for _index (range (`self.AmountOfBlocks`))
    (`self.AddBlock` (not (< _index 3)))))

(fn `AddBlock`
  (params (SpawnStuff :type Boolean :default true))
  (`|SpawnActorFromClass` "/Game/Blueprints/BP_Block.BP_Block_C" (`KismetMathLibrary.MakeTransform` (`KismetMathLibrary.MakeVector` (* (`self.LastBlock`) 800.0)) (struct :`Yaw` 180.0)) "Undefined" "OverrideRootScale" null SpawnStuff null)
  (`/Engine/EditorBlueprintResources/StandardMacros.IncrementInt` (`self.LastBlock`)))

(fn `UserConstructionScript`)