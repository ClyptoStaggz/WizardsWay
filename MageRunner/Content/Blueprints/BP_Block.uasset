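; Four-lane track block for the MageRunner runner game that randomly dresses itself with sidewalk and road obstacles, plus a coin pickup if a randomly picked lane is empty.
; A line trace finds the neighboring block to block road spawns in lanes holding rowboats.
; The two road obstacles move along -X each tick, and any obstacle overlap registers a player hit.
; Crossing the overlap box makes the game mode add a block, then this one self-destructs after a delay.
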(event `self.ReceiveBeginPlay`
  (bind _asbp_mage_runner (cast `/Game/Blueprints/BP_MageRunner` (`GameplayStatics.GetPlayerCharacter` 0)))
  (set `self.MageRunnerRef` _asbp_mage_runner)
  (bind _frontblock (`self.CheckFrontBlock`))
  (`/Engine/EditorBlueprintResources/StandardMacros.IsValid` _frontblock
    (:`Is Valid`
      (set `self.SpawnLane2Car` (not (== (`StaticMeshComponent.StaticMesh` (`/Game/Blueprints/BP_Block.Obstacle2` _frontblock)) "/Game/Imported/Fantastic_Village_Pack/meshes/props/vehicles/SM_PROP_rowboat.SM_PROP_rowboat")))
      (set `self.SpawnLane3Car` (not (== (`StaticMeshComponent.StaticMesh` (`/Game/Blueprints/BP_Block.Obstacle3` _frontblock)) "/Game/Imported/Fantastic_Village_Pack/meshes/props/vehicles/SM_PROP_rowboat.SM_PROP_rowboat"))))
    (:`Is Not Valid`
      _))
  (`self.SpawnObstacle`)
  (`self.SpawnCoins`))

(event `self.ReceiveTick`
  (params (DeltaSeconds :type "Float (single-precision)"))
  (`self.MoveObstacle` (`self.Obstacle2`) (`self.MovementSpeed`))
  (`self.MoveObstacle` (`self.Obstacle3`) (`self.MovementSpeed`)))

(event `self.OverlapBox.OnComponentBeginOverlap`
  (params (OverlappedComponent :type "PrimitiveComponent Object Reference") (OtherActor :type "Actor Object Reference") (OtherComp :type "PrimitiveComponent Object Reference") (OtherBodyIndex :type Integer) (bFromSweep :type Boolean) (SweepResult :type "HitResult Structure (by ref)"))
  (cast `/Game/Blueprints/BP_MageRunner` OtherActor)
  (bind _asgm_mage_runner (cast `/Game/Blueprints/GM_MageRunner` (`GameplayStatics.GetGameMode`)))
  (`/Game/Blueprints/GM_MageRunner.AddBlock` _asgm_mage_runner true)
  (`KismetSystemLibrary.Delay` 2.0)
  (`self.K2_DestroyActor`))

(event `self.Obstacle1.OnComponentBeginOverlap`
  (params (OverlappedComponent :type "PrimitiveComponent Object Reference") (OtherActor :type "Actor Object Reference") (OtherComp :type "PrimitiveComponent Object Reference") (OtherBodyIndex :type Integer) (bFromSweep :type Boolean) (SweepResult :type "HitResult Structure (by ref)"))
  (bind _asbp_mage_runner (cast `/Game/Blueprints/BP_MageRunner` OtherActor))
  (`self.AddHitToPlayer` _asbp_mage_runner))

(event `self.Obstacle2.OnComponentBeginOverlap`
  (params (OverlappedComponent :type "PrimitiveComponent Object Reference") (OtherActor :type "Actor Object Reference") (OtherComp :type "PrimitiveComponent Object Reference") (OtherBodyIndex :type Integer) (bFromSweep :type Boolean) (SweepResult :type "HitResult Structure (by ref)"))
  (bind _asbp_mage_runner (cast `/Game/Blueprints/BP_MageRunner` OtherActor))
  (`self.AddHitToPlayer` _asbp_mage_runner))

(event `self.Obstacle3.OnComponentBeginOverlap`
  (params (OverlappedComponent :type "PrimitiveComponent Object Reference") (OtherActor :type "Actor Object Reference") (OtherComp :type "PrimitiveComponent Object Reference") (OtherBodyIndex :type Integer) (bFromSweep :type Boolean) (SweepResult :type "HitResult Structure (by ref)"))
  (bind _asbp_mage_runner (cast `/Game/Blueprints/BP_MageRunner` OtherActor))
  (`self.AddHitToPlayer` _asbp_mage_runner))

(event `self.Obstacle4.OnComponentBeginOverlap`
  (params (OverlappedComponent :type "PrimitiveComponent Object Reference") (OtherActor :type "Actor Object Reference") (OtherComp :type "PrimitiveComponent Object Reference") (OtherBodyIndex :type Integer) (bFromSweep :type Boolean) (SweepResult :type "HitResult Structure (by ref)"))
  (bind _asbp_mage_runner (cast `/Game/Blueprints/BP_MageRunner` OtherActor))
  (`self.AddHitToPlayer` _asbp_mage_runner))

(fn `AddHitToPlayer`
  (params (PlayerRef :type "/Game/Blueprints/BP_MageRunner Object Reference"))
  (`/Engine/EditorBlueprintResources/StandardMacros.IncrementInt` (`/Game/Blueprints/BP_MageRunner.HitsTaken` PlayerRef)
    (:`  `
      (set `/Game/Blueprints/BP_MageRunner.SpringArmInterpSpeed` 5.0 PlayerRef)
      (`/Game/Blueprints/BP_MageRunner.WaitToRemoveHit` PlayerRef))))

(fn `CheckFrontBlock`
  (returns (FrontBlock :type "/Game/Blueprints/BP_Block Object Reference"))
  (bind _returnvalue (`self.K2_GetActorLocation`))
  (bind _outhit (`KismetSystemLibrary.LineTraceSingle` :`Start` _returnvalue :`End` (+ _returnvalue (* (`self.GetActorForwardVector`) -400.0)) :`TraceChannel` "TraceTypeQuery1" :`DrawDebugType` "ForDuration"))
  (bind _asbp_block (cast `/Game/Blueprints/BP_Block` (`.HitActor` (`GameplayStatics.BreakHitResult` _outhit))))
  (return _asbp_block))

(fn `MoveObstacle`
  (params (Target :type "SceneComponent Object Reference") (MovementSpeed :type "Float (single-precision)"))
  (`SceneComponent.K2_SetWorldLocation` Target (+ (`SceneComponent.K2_GetComponentLocation` Target) (* (-1.0 0.0 0.0) MovementSpeed)) false false))

(fn `SpawnCoins`
  (bind _output_get (set `self.CoinLane` (`KismetMathLibrary.RandomIntegerInRange` 0 3)))
  (bind _returnvalue (select `int` _output_get :`0` (`self.Obstacle1`) :`1` (`self.Obstacle2`) :`2` (`self.Obstacle3`) :`3` (`self.Obstacle4`)))
  (`/Engine/EditorBlueprintResources/StandardMacros.IsValid` (`StaticMeshComponent.StaticMesh` _returnvalue)
    (:`Is Not Valid`
      (`|SpawnActorFromClass` "/Game/Blueprints/Pickups/BP_Pickup_Coins.BP_Pickup_Coins_C" (`KismetMathLibrary.MakeTransform` (`SceneComponent.K2_GetComponentLocation` _returnvalue)) "Undefined" "OverrideRootScale" null null))))

(fn `SpawnObstacle`
  (if (`self.SpawnStuff`)
    (if (`self.CalcRandom` 0 1)
      (`|ExecutionSequence`
        (:`then_0`
          (if (`self.CalcRandom` 0 1)
            (`StaticMeshComponent.SetStaticMesh` (`self.Obstacle1`) (`KismetArrayLibrary.Array_Random` (`self.SidewalkMeshes`)))))
        (:`then_1`
          ;[1 1 1] Checks to see if valid spot to spawn
          (if (`self.SpawnLane2Car`)
            (if (`self.CalcRandom` 0 1)
              (`StaticMeshComponent.SetStaticMesh` (`self.Obstacle2`) (`KismetArrayLibrary.Array_Random` (`self.RoadMeshes`))))))
        (:`then_2`
          (if (`self.SpawnLane3Car`)
            (if (`self.CalcRandom` 0 1)
              (`StaticMeshComponent.SetStaticMesh` (`self.Obstacle3`) (`KismetArrayLibrary.Array_Random` (`self.RoadMeshes`))))))
        (:`then_3`
          (if (`self.CalcRandom` 0 1)
            (`StaticMeshComponent.SetStaticMesh` (`self.Obstacle4`) (`KismetArrayLibrary.Array_Random` (`self.SidewalkMeshes`)))))))))

(fn `UserConstructionScript`)