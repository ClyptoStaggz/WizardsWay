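; BP_MageRunner is an auto-running player character that switches lanes sideways and jumps, in the style of an endless runner.
; Left and Right presses step a target world Y by a fixed lane width, clamped by rejecting moves past the track bounds.
; Each Tick adds forward movement input and eases Y toward that target with FInterpTo and SetActorLocation, while Jump uses the built-in Character jump.
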(event `self.ReceiveBeginPlay`
  (bind (_returnvalue_x _returnvalue_y) (`KismetMathLibrary.BreakVector` (`self.K2_GetActorLocation`)))
  (set `self.TargetY` _returnvalue_y))

(event `InputAction|MoveRight`
  (params (Key :type "Key Structure"))
  (bind _returnvalue (+ (`self.TargetY`) 400.0))
  ;[0.05098 0.05098 0.05098] Movement Input - Move Left / Right and Jump
  ; See Project Settings -> Input for Action and Axis Mappings
  ; Jump Input - Jump can be configured in the CharacterMovementComponent
  (:`Pressed`
    (if (not (> _returnvalue 1450.0))
      (set `self.TargetY` _returnvalue))))

(event `InputAction|MoveLeft`
  (params (Key :type "Key Structure"))
  (bind _returnvalue (+ (`self.TargetY`) -400.0))
  ;[0.05098 0.05098 0.05098] Movement Input - Move Left / Right and Jump
  ; See Project Settings -> Input for Action and Axis Mappings
  ; Jump Input - Jump can be configured in the CharacterMovementComponent
  (:`Pressed`
    (if (not (< _returnvalue 150.0))
      (set `self.TargetY` _returnvalue))))

(event `InputAction|Slide`
  (params (Key :type "Key Structure"))
  ;[0.05098 0.05098 0.05098] Movement Input - Move Left / Right and Jump
  ; See Project Settings -> Input for Action and Axis Mappings
  ; Jump Input - Jump can be configured in the CharacterMovementComponent
)

(event `InputAction|Jump` :overrideparent false
  (params (Key :type "Key Structure"))
  ;[0.05098 0.05098 0.05098] Movement Input - Move Left / Right and Jump
  ; See Project Settings -> Input for Action and Axis Mappings
  ; Jump Input - Jump can be configured in the CharacterMovementComponent
  (:`Pressed`
    (`self.Jump`))
  (:`Released`
    (`self.StopJumping`)))

(event `self.ReceiveTick`
  (params (DeltaSeconds :type "Float (single-precision)"))
  (bind (_returnvalue_x _returnvalue_y _returnvalue_z) (`KismetMathLibrary.BreakVector` (`self.K2_GetActorLocation`)))
  (`self.AddMovementInput` (`self.GetActorForwardVector`))
  (`self.K2_SetActorLocation` (`KismetMathLibrary.MakeVector` _returnvalue_x (`KismetMathLibrary.FInterpTo` _returnvalue_y (`self.TargetY`) DeltaSeconds 10.0) _returnvalue_z)))

(fn `UserConstructionScript`)