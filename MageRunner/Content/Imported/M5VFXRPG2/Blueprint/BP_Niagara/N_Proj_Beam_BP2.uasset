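; Niagara beam projectile actor that draws a timed beam effect between a source and a target point, then removes itself.
; Proj_PT_Set receives the fire, beam and explosion systems, both endpoints and the duration, then assigns them to three Niagara components.
; Tick feeds the beam's Start/End parameters and pins the explosion to the target until a Delay ends the beam, then deactivates all three and destroys the actor after another delay.
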(event `self.ReceiveTick`
  (params (DeltaSeconds :type "Float (single-precision)"))
  (bind _targetlocation (`self.TargetLocation`))
  (bind _n_proj_pt (`self.N_Proj_PT`))
  ;[1 1 1] Beam
  (if (`self.beamcontinue`)
    (`ActorComponent.SetActive` (`self.N_Proj_PT`) true false)
    (`ActorComponent.SetActive` (`self.N_ProjExp_PT`) true false)
    (`ActorComponent.SetActive` (`self.N_ProjFire_PT`) true false)
    (`NiagaraComponent.SetVariablePosition` _n_proj_pt "Start" (`self.SourceLocation`))
    (`NiagaraComponent.SetVariablePosition` _n_proj_pt "End" _targetlocation)
    (`SceneComponent.K2_SetWorldLocation` (`self.N_ProjExp_PT`) _targetlocation false true)
    (`KismetSystemLibrary.Delay` (`self.BeamContinueTime`))
    (set `self.beamcontinue` false)
    (else
      (`ActorComponent.SetActive` (`self.N_Proj_PT`) false false)
      (`ActorComponent.SetActive` (`self.N_ProjExp_PT`) false false)
      (`ActorComponent.SetActive` (`self.N_ProjFire_PT`) false false)
      (`KismetSystemLibrary.Delay` 2.0)
      (`self.K2_DestroyActor`))))

(event `Proj_PT_Set`
  (params (ProjectileFire_PT :type "NiagaraSystem Object Reference") (projectile_PT :type "NiagaraSystem Object Reference") (ProjectileExplosion_PT :type "NiagaraSystem Object Reference") (TargetPoint :type "Vector Structure") (SourcePoint :type "Vector Structure") (beamContinue :type Boolean) (BeamContinuetime :type "Float (double-precision)"))
  (bind _n_proj_pt (`self.N_Proj_PT`))
  (bind _n_projfire_pt (`self.N_ProjFire_PT`))
  ;[1 1 1] Projectile Particle
  (set `self.BeamContinueTime` BeamContinuetime)
  (bind _output_get (set `self.beamcontinue` beamContinue))
  (if _output_get
    (set `self.SourceLocation` SourcePoint)
    (set `self.TargetLocation` TargetPoint)
    (`SceneComponent.K2_SetWorldLocation` _n_projfire_pt (`self.SourceLocation`) false true)
    (`NiagaraComponent.SetAsset` _n_projfire_pt ProjectileFire_PT true)
    (`NiagaraComponent.SetAsset` (`self.N_ProjExp_PT`) ProjectileExplosion_PT true)
    (`NiagaraComponent.SetAsset` (`self.N_Proj_PT`) projectile_PT true)
    (`NiagaraComponent.SetVariablePosition` _n_proj_pt "Start" (`self.SourceLocation`))
    (`NiagaraComponent.SetVariablePosition` _n_proj_pt "End" (`self.TargetLocation`))))

(fn `UserConstructionScript`)